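; BP_Projectile_Fireball is an enemy fireball projectile that damages sidescroller characters on impact and explodes.
; BeginPlay rotates its initial velocity to the actor's facing, attaches a sound and ignores its instigator.
; A hit applies damage without knockback, sets a replicated explosion transform slightly behind the impact and destroys the actor.
; That transform's RepNotify spawns a small BP_Explosion; HitWithAttack always returns false.
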(event `self.ReceiveBeginPlay`
  (set `MovementComponent.Velocity` (`KismetMathLibrary.GreaterGreater_VectorRotator` (`self.Initial Velocity`) (`self.K2_GetActorRotation`)) (`self.Projectile component`))
  (`GameplayStatics.SpawnSoundAttached` "/Game/ExampleContent/Audio/Room_03/Arcade_Enemy_Destroyed_Cue.Arcade_Enemy_Destroyed_Cue" (`self.Fireball`) "None" (0.0 0.0 0.0) (struct) "EAttachLocation::KeepRelativeOffset" false 1.0 1.0)
  (`PrimitiveComponent.IgnoreActorWhenMoving` (`self.Fireball`) (`self.GetInstigator`) true))

(event `self.ReceiveHit`
  (params (MyComp :type "PrimitiveComponent Object Reference") (Other :type "Actor Object Reference") (OtherComp :type "PrimitiveComponent Object Reference") (bSelfMoved :type Boolean) (HitLocation :type "Vector Structure") (HitNormal :type "Vector Structure") (NormalImpulse :type "Vector Structure") (Hit :type "HitResult Structure (by ref)"))
  (if (!= Other (`self.GetInstigator`))
    (bind _assidescroller_character (cast `/Game/Sidescroller/SidescrollerCharacter` Other)
      (:`then`
        (`/Game/Sidescroller/SidescrollerCharacter.ApplyDamage` _assidescroller_character 5.0 0.0 self))
      (:`CastFailed`
        _))
    (`/Engine/EditorBlueprintResources/ActorMacros.Switch Has Authority`
      (:`Authority`
        _)
      (:`Remote`
        _))
    (set `self.Rep_ExplosionTransform` (`KismetMathLibrary.MakeTransform` (+ (`self.K2_GetActorLocation`) (* (`KismetMathLibrary.Conv_RotatorToVector` (`self.K2_GetActorRotation`)) -20.0))))
    (`self.K2_DestroyActor`)))

(fn `Hit with attack`
  (params (`Impact vector` :type "Vector Structure") (`Weapon damage` :type "Float (double-precision)") (`Weapon weight` :type "Float (double-precision)") (Attacker :type "Actor Object Reference"))
  (returns (bWasDamaged :type Boolean))
  (return false))

(fn `OnRep_Rep_ExplosionTransform`
  (`|SpawnActorFromClass` "/Game/Blueprints/Game/BP_Explosion.BP_Explosion_C" (`self.Rep_ExplosionTransform`) "AlwaysSpawn" "OverrideRootScale" null (`self.SMall explosion`) (`self.Owner_0`)))

(fn `UserConstructionScript`)