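; Bullet-hell projectile actor that draws a swarm of about two thousand small projectiles through one InstancedStaticMesh.
; BeginPlay spawns the scaled-down instances at the actor origin and stores random planar velocities, which movement never uses.
; Tick nudges each instance by a fresh random XY offset in world space, giving frame-rate-dependent jitter.
; Only one mid-loop update (index 100) marks render state dirty, avoiding a refresh per instance.
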(event `self.ReceiveBeginPlay`
  (for _ (range 2001)
    (`InstancedStaticMeshComponent.AddInstance` (`self.InstancedStaticMesh`) (`KismetMathLibrary.MakeTransform` (0.0 0.0 0.0) (struct) (0.2 0.2 0.2)))
    (`KismetArrayLibrary.Array_Add` (`self.RandomVectorVel`) (* (`KismetMathLibrary.MakeVector` (.x (`KismetMathLibrary.RandomUnitVector`)) (.y (`KismetMathLibrary.RandomUnitVector`))) 10.0))))

(event `self.ReceiveTick`
  (params (DeltaSeconds :type "Float (single-precision)"))
  (bind _instancedstaticmesh (`self.InstancedStaticMesh`))
  (for _index (range 2001)
    (bind _outinstancetransform (`InstancedStaticMeshComponent.GetInstanceTransform` _instancedstaticmesh _index true))
    (`InstancedStaticMeshComponent.UpdateInstanceTransform` _instancedstaticmesh _index (`KismetMathLibrary.MakeTransform` (+ (`KismetMathLibrary.MakeVector` (.x (`KismetMathLibrary.RandomUnitVector`)) (.y (`KismetMathLibrary.RandomUnitVector`))) (.location _outinstancetransform)) (.rotation _outinstancetransform) (.scale _outinstancetransform)) true (== _index 100) false)))

(fn `UserConstructionScript`)