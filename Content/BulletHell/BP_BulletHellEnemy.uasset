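; Pooled bullet-hell enemy that flies a randomized path while firing pooled projectiles at random players.
; ConstructSpline threads its start through four distinct random "Inner" actors to a random "Outer" one, and a timeline moves it along that spline.
; A looping timer feeds a DoN-gated burst, with pattern type setting cadence and tint.
; Projectile hits drain health until it explodes; death or any other hit returns it to BP_Pool.
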(event `ConstructSpline`
  (bind _returnvalue (`KismetMathLibrary.RandomIntegerInRange` 0 5))
  (bind _foundtargetpoints (`self.FoundTargetPoints`))
  (bind _foundtargetpoints_2 (`self.FoundTargetPoints`))
  (bind _spline (`self.Spline`))
  (`SplineComponent.ClearSplinePoints` _spline true)
  (`KismetArrayLibrary.Array_Clear` _foundtargetpoints)
  (`SplineComponent.AddSplinePoint` _spline (`self.StartPosition`) "World" true)
  (while (< (`KismetArrayLibrary.Array_Length` _foundtargetpoints) 4)
    (if (not (`KismetArrayLibrary.Array_Contains` _foundtargetpoints_2 _returnvalue))
      (`KismetArrayLibrary.Array_Add` _foundtargetpoints_2 _returnvalue)))
  (bind _outactors (`GameplayStatics.GetAllActorsWithTag` "Inner"))
  (for _array_element (`self.FoundTargetPoints`)
    (`SplineComponent.AddSplinePoint` _spline (`self.K2_GetActorLocation` (`|GetArrayItem` _outactors _array_element)) "World" true))
  (bind _outactors_2 (`GameplayStatics.GetAllActorsWithTag` "Outer"))
  (`SplineComponent.AddSplinePoint` _spline (`self.K2_GetActorLocation` (`|GetArrayItem` _outactors_2 (`KismetMathLibrary.RandomIntegerInRange` 0 (- (`KismetArrayLibrary.Array_Length` _outactors_2) 1)))) "World" true))

(event `ActivateTimeline`
  (bind _spline (`self.Spline`))
  (`|ExecutionSequence`
    (:`then_0`
      (bind _returnvalue (`KismetSystemLibrary.K2_SetTimerDelegate` (delegate `ShootBullets`) (select `/Game/BulletHell/Enum_BulletPattern` (`self.PatternType`) :`NewEnumerator0` 1.0 :`NewEnumerator1` 0.1) true)))
    (:`then_1`
      (bind (_direction _newtrack_5) (`Timeline|SplineMovement` :!via `PlayFromStart` :!label _label)
        (:`Update`
          (`self.K2_SetActorLocation` (+ (`SplineComponent.GetLocationAtDistanceAlongSpline` _spline (* _newtrack_5 (`SplineComponent.GetSplineLength` _spline)) "Local") (`self.StartPosition`)) true))))))

(event `StopTimeline`
  (`|ExecutionSequence`
    (:`then_0`
      (`KismetSystemLibrary.K2_ClearAndInvalidateTimerHandle` (stale `ActivateTimeline` _returnvalue)))
    (:`then_1`
      (goto _label :!via `Stop`))))

(event `ShootBullets`
  (`/Engine/EditorBlueprintResources/StandardMacros.Do N` (select `/Game/BulletHell/Enum_BulletPattern` (`self.PatternType`) :`NewEnumerator0` 10 :`NewEnumerator1` 10) :!label _label_2
    (:`Exit`
      (`self.Shoot`)
      (`KismetSystemLibrary.Delay` (select `/Game/BulletHell/Enum_BulletPattern` (`self.PatternType`) :`NewEnumerator0` 1.0 :`NewEnumerator1` 4.0))
      (goto _label_2 :!via `Reset`))))

(event `self.ReceiveBeginPlay`
  (`KismetSystemLibrary.Delay` 0.2)
  (bind _outactors (`GameplayStatics.GetAllActorsOfClass` "/Game/BulletHell/BP_Pool.BP_Pool_C"))
  (set `self.Pool` (`|GetArrayItem` _outactors))
  (bind _outactors_2 (`GameplayStatics.GetAllActorsOfClass` "/Game/BulletHell/BP_BulletHellCharacter.BP_BulletHellCharacter_C"))
  (for _array_element _outactors_2
    (`KismetArrayLibrary.Array_Add` (`self.PlayerList`) _array_element)
    (`KismetSystemLibrary.Delay` 2.0)))

(event `self.ReceiveHit`
  (params (MyComp :type "PrimitiveComponent Object Reference") (Other :type "Actor Object Reference") (OtherComp :type "PrimitiveComponent Object Reference") (bSelfMoved :type Boolean) (HitLocation :type "Vector Structure") (HitNormal :type "Vector Structure") (NormalImpulse :type "Vector Structure") (Hit :type "HitResult Structure (by ref)"))
  (bind _pool (`self.Pool`))
  (if (`KismetMathLibrary.ClassIsChildOf` (`GameplayStatics.GetObjectClass` Other) "/Game/BulletHell/BP_Projectile.BP_Projectile_C")
    (bind _result (`/Engine/EditorBlueprintResources/StandardMacros.DecrementFloat` (`self.Health`))
      (:`  `
        (bind _output_get (set `self.Health` _result))
        (if (<= _output_get 0.0)
          (`GameplayStatics.SpawnEmitterAtLocation` "/Game/Effects/Particle_Systems/P_Explosion_Fireball.P_Explosion_Fireball" HitLocation)
          (set `self.isShooting` false)
          (`self.StopTimeline`)
          (`/Game/BulletHell/BP_Pool.AddEnemyToPool` _pool self))))
    (else
      (`self.StopTimeline`)
      (set `self.isShooting` false)
      (`/Game/BulletHell/BP_Pool.AddEnemyToPool` _pool self))))

(fn `OnRep_Health`)

(fn `SetType`
  (params (NewPattern :type "/Game/BulletHell/Enum_BulletPattern Enum" :default "NewEnumerator0"))
  (bind _matinstance (`self.MatInstance`))
  (set `self.PatternType` NewPattern)
  (switch `/Game/BulletHell/Enum_BulletPattern` NewPattern
    (:`NewEnumerator0`
      (`MaterialInstanceDynamic.SetVectorParameterValue` _matinstance "Base Color" (struct :`R` 0.653448 :`G` 0.627056 :`B` 0.565536 :`A` 1.0)))
    (:`NewEnumerator1`
      (`MaterialInstanceDynamic.SetVectorParameterValue` _matinstance "Base Color" (struct :`R` 1.0 :`G` 0.005 :`A` 1.0)))))

(fn `Shoot`
  (bind _returnvalue (`self.K2_GetActorLocation`))
  (bind _playerlist (`self.PlayerList`))
  (if (`self.isShooting`)
    (switch `/Game/BulletHell/Enum_BulletPattern` (`self.PatternType`)
      (:`NewEnumerator0`
        _)
      (:`NewEnumerator1`
        _))
    (bind (_projectile _issuccessful) (`/Game/BulletHell/BP_Pool.GetBulletFromPool` (`self.Pool`) true))
    (if _issuccessful
      (`/Game/BulletHell/BP_Projectile.ActivateBullet` _projectile (* (`KismetMathLibrary.Normal` (- (`self.K2_GetActorLocation` (`|GetArrayItem` _playerlist (`KismetMathLibrary.RandomIntegerInRange` 0 (- (`KismetArrayLibrary.Array_Length` _playerlist) 1)))) _returnvalue)) 500.0) (+ (0.0 0.0 0.0) _returnvalue)))))

(fn `UserConstructionScript`
  (set `self.StartPosition` (`self.K2_GetActorLocation`))
  (bind _returnvalue (`PrimitiveComponent.CreateDynamicMaterialInstance` (`self.StaticMesh`) 0 "/Game/ExampleContent/Input_Examples/Materials/M_Toy_Cow.M_Toy_Cow" "None"))
  (set `self.MatInstance` _returnvalue))