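; Player character for the bullet-hell game, handling firing, lives and respawn.
; Firing reuses projectiles from a passed-in pool, launching them along +X through RPC-to-Multi event pairs, a pattern also used for hits.
; Enemy projectile hits decrement lives on the controller's HUD, then either open the main menu or explode, hide and respawn the character at a fixed point with input restored and brief invulnerability.
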(event `self.ReceiveBeginPlay`)

(event `RPCHit`
  (`self.MultiHit`))

(event `MultiHit`
  (if (not (`self.Invulnerable`))
    (set `self.Invulnerable` true)
    (bind _asbp_bullet_hell_player_controller (cast `/Game/BulletHell/BP_BulletHellPlayerController` (`self.GetController`)))
    (bind _result (`/Engine/EditorBlueprintResources/StandardMacros.DecrementInt` (`self.LiveCount`))
      (:`  `
        (if (<= _result 0)
          (bind _lives (`/Game/BulletHell/BulletCount.Lives` (`/Game/BulletHell/BP_BulletHellPlayerController.BulletBar` _asbp_bullet_hell_player_controller)))
          (bind _returnvalue (`KismetTextLibrary.Conv_IntToText` _result))
          (`TextBlock.SetText` _lives _returnvalue)
          (`GameplayStatics.OpenLevel` "MainMenu")
          (else
            (`TextBlock.SetText` _lives _returnvalue)
            (`self.SetActorEnableCollision` true)
            (`self.SetActorHiddenInGame` true)
            (`GameplayStatics.SpawnEmitterAtLocation` "/Game/ExampleContent/Blueprint_Communication/Effects/P_Explosion_Fireball.P_Explosion_Fireball" (`self.K2_GetActorLocation`))
            (set `/Game/Blueprints/BP_PlayerController.isInputActive` false _asbp_bullet_hell_player_controller)
            (`KismetSystemLibrary.Delay` 2.0)
            (`self.K2_SetActorLocation` (-400.0 0.0 0.0))
            (`self.SetActorEnableCollision` true)
            (`self.SetActorHiddenInGame` false)
            (set `/Game/Blueprints/BP_PlayerController.isInputActive` true _asbp_bullet_hell_player_controller)
            (set `self.Invulnerable` true)
            (`KismetSystemLibrary.Delay` 2.0)
            (set `self.Invulnerable` false)))))))

(event `self.ReceiveTick`
  (params (DeltaSeconds :type "Float (single-precision)")))

(event `self.ReceiveHit`
  (params (MyComp :type "PrimitiveComponent Object Reference") (Other :type "Actor Object Reference") (OtherComp :type "PrimitiveComponent Object Reference") (bSelfMoved :type Boolean) (HitLocation :type "Vector Structure") (HitNormal :type "Vector Structure") (NormalImpulse :type "Vector Structure") (Hit :type "HitResult Structure (by ref)"))
  (if (`KismetMathLibrary.ClassIsChildOf` (`GameplayStatics.GetObjectClass` Other) "/Game/BulletHell/BP_Projectile_Enemy.BP_Projectile_Enemy_C")
    (`self.RPCHit`)))

(event `RPCFireProjectile`
  (params (Pool :type "/Game/BulletHell/BP_Pool Object Reference"))
  (`self.MultiFireProjectile` Pool))

(event `MultiFireProjectile`
  (params (Pool :type "/Game/BulletHell/BP_Pool Object Reference"))
  (bind (_projectile _issuccessful) (`/Game/BulletHell/BP_Pool.GetBulletFromPool` Pool false))
  (if _issuccessful
    (`self.SetActorHiddenInGame` _projectile false)
    (`self.SetActorEnableCollision` _projectile true)
    (bind _projectilemovement (`/Game/BulletHell/BP_Projectile.ProjectileMovement` _projectile))
    (`ActorComponent.Activate` _projectilemovement false)
    (`self.K2_SetActorLocation` _projectile (+ (`self.K2_GetActorLocation`) (100.0 0.0 0.0) (0.0 0.0 0.0)) false false)
    (set `MovementComponent.Velocity` (1000.0 0.0 0.0) _projectilemovement)
    (else
      (`KismetSystemLibrary.PrintString` "empty storage"))))

(fn `UserConstructionScript`)