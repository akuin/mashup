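; BP_Pool is an object pool for a bullet hell game, holding player bullets, enemy bullets and enemies.
; Shortly after BeginPlay it pre-spawns all three sets hidden, with collision and tick disabled, into storage arrays.
; Get functions hand out the first stored actor; add functions return it, with only enemies being hidden and moved away here.
; Enemy bullets are also tracked as active, feeding an in-use count to the BulletCount widget.
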(event `self.ReceiveBeginPlay`
  (`KismetSystemLibrary.Delay` 0.2)
  (for _ (range (+ (`self.PlayerBulletCount`) 1))
    (bind _returnvalue (`|SpawnActorFromClass` "/Game/BulletHell/BP_Projectile_Player.BP_Projectile_Player_C" (`KismetMathLibrary.MakeTransform` (0.0 0.0 100.0) (struct :`Yaw` -500.0) (0.2 0.2 0.2)) "AlwaysSpawn" "OverrideRootScale" null null))
    (`self.SetActorEnableCollision` _returnvalue false)
    (`self.SetActorHiddenInGame` _returnvalue true)
    (`self.SetActorTickEnabled` _returnvalue false)
    (`KismetArrayLibrary.Array_Add` (`self.PlayerBulletStorage`) _returnvalue))
  (for _ (range (+ (`self.EnemyBulletCount`) 1))
    (bind _returnvalue_2 (`|SpawnActorFromClass` "/Game/BulletHell/BP_Projectile_Enemy.BP_Projectile_Enemy_C" (`KismetMathLibrary.MakeTransform` (0.0 0.0 100.0) (struct) (0.3 0.3 0.3)) "AlwaysSpawn" "OverrideRootScale" null null))
    (`self.SetActorEnableCollision` _returnvalue_2 false)
    (`self.SetActorHiddenInGame` _returnvalue_2 true)
    (`self.SetActorTickEnabled` _returnvalue_2 false)
    (`KismetArrayLibrary.Array_Add` (`self.EnemyBulletStorage`) _returnvalue_2))
  (bind _foundwidgets (`WidgetBlueprintLibrary.GetAllWidgetsOfClass` "/Game/BulletHell/BulletCount.BulletCount_C"))
  (set `self.BulletWidget` (`|GetArrayItem` _foundwidgets))
  (for _ (range (+ (`self.EnemyCount`) 1))
    (bind _returnvalue_3 (`|SpawnActorFromClass` "/Game/BulletHell/BP_BulletHellEnemy.BP_BulletHellEnemy_C" (`KismetMathLibrary.MakeTransform` (0.0 0.0 100.0) (struct) (1.0 1.0 1.0)) "AlwaysSpawn" "OverrideRootScale" null null))
    (`self.SetActorEnableCollision` _returnvalue_3 false)
    (`self.SetActorHiddenInGame` _returnvalue_3 true)
    (`self.SetActorTickEnabled` _returnvalue_3 false)
    (`KismetArrayLibrary.Array_Add` (`self.EnemyStorage`) _returnvalue_3)))

(fn `AddBulletToPool`
  (params (Projectile :type "/Game/BulletHell/BP_Projectile Object Reference"))
  (if (== (`GameplayStatics.GetObjectClass` Projectile) "/Game/BulletHell/BP_Projectile_Player.BP_Projectile_Player_C")
    (`KismetArrayLibrary.Array_Add` (`self.PlayerBulletStorage`) Projectile)
    (else
      (`KismetArrayLibrary.Array_RemoveItem` (`self.ActiveBullets`) Projectile)
      (`KismetArrayLibrary.Array_Add` (`self.EnemyBulletStorage`) Projectile)
      (bind _result (`/Engine/EditorBlueprintResources/StandardMacros.DecrementInt` (`self.BulletsInUse`))
        (:`  `
          (bind _output_get (set `self.BulletsInUse` _result))
          (`/Game/BulletHell/BulletCount.UpdateBulletCount` (`self.BulletWidget`) _output_get))))))

(fn `AddEnemyToPool`
  (params (Enemy :type "/Game/BulletHell/BP_BulletHellEnemy Object Reference"))
  (`self.SetActorEnableCollision` Enemy false)
  (`self.SetActorHiddenInGame` Enemy true)
  (`self.K2_SetActorLocation` Enemy (0.0 0.0 -1000.0) false true)
  (`KismetArrayLibrary.Array_Add` (`self.EnemyStorage`) Enemy))

(fn `GetBulletFromPool`
  (params (isEnemy :type Boolean))
  (returns (Projectile :type "/Game/BulletHell/BP_Projectile Object Reference") (isSuccessful :type Boolean))
  (locals (TempBulllet :type "/Game/BulletHell/BP_Projectile Object Reference"))
  (bind _playerbulletstorage (`self.PlayerBulletStorage`))
  (bind _enemybulletstorage (`self.EnemyBulletStorage`))
  (if isEnemy
    (bind _output_get (set `local.TempBulllet` (`|GetArrayItem` _enemybulletstorage)))
    (bind _returnvalue (`KismetArrayLibrary.Array_RemoveItem` _enemybulletstorage _output_get))
    (if _returnvalue
      (bind _result (`/Engine/EditorBlueprintResources/StandardMacros.IncrementInt` (`self.BulletsInUse`))
        (:`  `
          (`/Game/BulletHell/BulletCount.UpdateBulletCount` (`self.BulletWidget`) _result)
          (`KismetArrayLibrary.Array_Add` (`self.ActiveBullets`) _output_get))))
    (return _output_get _returnvalue)
    (else
      (bind _output_get_2 (set `local.TempBulllet` (`|GetArrayItem` _playerbulletstorage)))
      (bind _returnvalue_2 (`KismetArrayLibrary.Array_RemoveItem` _playerbulletstorage _output_get_2))
      (return _output_get_2 _returnvalue_2))))

(fn `GetEnemyFromPool`
  (returns (Enemy :type "/Game/BulletHell/BP_BulletHellEnemy Object Reference") (isSuccessful :type Boolean))
  (locals (TempBulllet :type "/Game/BulletHell/BP_BulletHellEnemy Object Reference"))
  (bind _enemystorage (`self.EnemyStorage`))
  (bind _output_get (set `local.TempBulllet` (`|GetArrayItem` _enemystorage)))
  (bind _returnvalue (`KismetArrayLibrary.Array_RemoveItem` _enemystorage _output_get))
  (return _output_get _returnvalue))

(fn `UserConstructionScript`)