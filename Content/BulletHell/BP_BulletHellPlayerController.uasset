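; Player controller for the bullet hell mode that moves the pawn along world axes and drives automatic firing.
; On local BeginPlay it shows the BulletCount widget, switches view to BP_BulletHellCamera and caches BP_Pool.
; Holding left mouse runs a gated 0.1-second loop calling RPCFireProjectile on BP_BulletHellCharacter with that pool.
; IsInputActive gates movement and firing; look, turn and jump only reach empty delays.
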(event `InputAxis|MoveForward`
  (params (AxisValue :type "Float (single-precision)"))
  (bind _returnvalue (`self.K2_GetPawn`))
  (if (`self.isInputActive`)
    (`/Engine/EditorBlueprintResources/StandardMacros.IsValid` _returnvalue
      (:`Is Valid`
        (`Pawn.AddMovementInput` _returnvalue (1.0 0.0 0.0) AxisValue false)))))

(event `InputAxis|LookUp`
  (params (AxisValue :type "Float (single-precision)"))
  (`KismetSystemLibrary.Delay` 0.0 :!label _label))

(event `InputAxis|Turn`
  (params (AxisValue :type "Float (single-precision)"))
  (goto _label))

(event `InputAxis|MoveRight` :consume false :overrideparent false
  (params (AxisValue :type "Float (single-precision)"))
  (bind _returnvalue (`self.K2_GetPawn`))
  (if (`self.isInputActive`)
    (`/Engine/EditorBlueprintResources/StandardMacros.IsValid` _returnvalue
      (:`Is Valid`
        (`Pawn.AddMovementInput` _returnvalue (0.0 1.0 0.0) AxisValue false)))))

(event `InputAction|Jump`
  (params (Key :type "Key Structure"))
  (:`Pressed`
    (`KismetSystemLibrary.Delay` 0.0 :!label _label_2))
  (:`Released`
    (goto _label_2)))

(event `self.ReceiveBeginPlay`
  (`parent.ReceiveBeginPlay`)
  (if (`self.IsLocalController`)
    (bind _returnvalue (`|CreateWidget` "/Game/BulletHell/BulletCount.BulletCount_C"))
    (set `self.BulletBar` _returnvalue)
    (`UserWidget.AddToViewport` _returnvalue 0)
    (`KismetSystemLibrary.Delay` 0.2)
    (bind _outactors (`GameplayStatics.GetAllActorsOfClass` "/Game/BulletHell/BP_BulletHellCamera.BP_BulletHellCamera_C"))
    (`self.SetViewTargetWithBlend` (`|GetArrayItem` _outactors))
    (bind _outactors_2 (`GameplayStatics.GetAllActorsOfClass` "/Game/BulletHell/BP_Pool.BP_Pool_C"))
    (set `self.BulletPool` (`|GetArrayItem` _outactors_2))
    (`KismetSystemLibrary.Delay` 1.0)
    (bind _outactors_3 (`GameplayStatics.GetAllActorsOfClass` "/Game/BulletHell/BP_BulletHellCamera.BP_BulletHellCamera_C"))
    (`self.SetViewTargetWithBlend` (`|GetArrayItem` _outactors_3))))

(event `Fire`
  (if (`self.isInputActive`)
    (bind _asbp_bullet_hell_character (cast `/Game/BulletHell/BP_BulletHellCharacter` (`self.K2_GetPawn`)))
    (`/Game/BulletHell/BP_BulletHellCharacter.RPCFireProjectile` _asbp_bullet_hell_character (`self.BulletPool`))
    (else
      (goto _label_3 :!via `Close`))))

(event `Key|LeftMouseButton`
  (params (Key :type "Key Structure"))
  (:`Pressed`
    (if (`self.isInputActive`)
      (`|ExecutionSequence`
        (:`then_0`
          (goto _label_3 :!via `Open`))
        (:`then_1`
          (`/Engine/EditorBlueprintResources/StandardMacros.Gate` true :!label _label_3
            (:`Exit`
              (`self.Fire`)
              (`KismetSystemLibrary.RetriggerableDelay` 0.1)
              (goto _label_3)))))))
  (:`Released`
    (goto _label_3 :!via `Close`)))

(fn `UserConstructionScript`)