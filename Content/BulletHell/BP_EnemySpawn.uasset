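; Bullet-hell enemy spawn area that places pooled enemies at random points inside its box.
; SpawnEnemy takes an enemy from the given pool, applies the pattern, re-enables collision and visibility, then starts its timeline, spline and shooting.
; Location and StartPosition are randomized separately, so they can differ.
; An empty pool only prints a failure; a direct SpawnActor path is left unconnected.
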(event `SpawnEnemy`
  (params (Pool :type "/Game/BulletHell/BP_Pool Object Reference") (Pattern :type "/Game/BulletHell/Enum_BulletPattern Enum" :default "NewEnumerator0"))
  (bind _returnvalue (`KismetMathLibrary.RandomPointInBoundingBox` (`self.K2_GetActorLocation`) (`BoxComponent.GetScaledBoxExtent` (`self.Box`))))
  (bind (_enemy _issuccessful) (`/Game/BulletHell/BP_Pool.GetEnemyFromPool` Pool))
  (if _issuccessful
    (`self.K2_SetActorLocation` _enemy _returnvalue false false)
    (set `/Game/BulletHell/BP_BulletHellEnemy.StartPosition` _returnvalue _enemy)
    (`/Game/BulletHell/BP_BulletHellEnemy.SetType` _enemy Pattern)
    (`self.SetActorEnableCollision` _enemy true)
    (`self.SetActorHiddenInGame` _enemy false)
    (`/Game/BulletHell/BP_BulletHellEnemy.ActivateTimeline` _enemy)
    (`/Game/BulletHell/BP_BulletHellEnemy.ConstructSpline` _enemy)
    (set `/Game/BulletHell/BP_BulletHellEnemy.isShooting` true _enemy)
    (else
      (`KismetSystemLibrary.PrintString` "failed"))))

(event `self.ReceiveBeginPlay`)

(fn `UserConstructionScript`)