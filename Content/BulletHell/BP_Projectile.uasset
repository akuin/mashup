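; Pooled bullet-hell projectile that is reused through BP_Pool, found on BeginPlay, rather than destroyed.
; ActivateBullet shows and launches it; Hit hides it, parks it below the world and returns it to the pool.
; Freeze nearly halts it, then scatters it horizontally at random.
; SlowDown briefly enables Tick-based deceleration, then aims it at the supplied player position.
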(event `Freeze`
  (bind (_returnvalue_x _returnvalue_y) (`KismetMathLibrary.BreakVector` (`KismetMathLibrary.RandomUnitVector`)))
  (bind _projectilemovement (`self.ProjectileMovement`))
  (set `MovementComponent.Velocity` (0.001 0.0 0.0) _projectilemovement)
  (`KismetSystemLibrary.Delay` 2.0)
  (set `MovementComponent.Velocity` (* (`KismetMathLibrary.Normal` (`KismetMathLibrary.MakeVector` _returnvalue_x _returnvalue_y)) (`KismetMathLibrary.RandomFloatInRange` 100.0 150.0)) _projectilemovement))

(event `SlowDown`
  (params (PlayerPosition :type "Vector Structure"))
  (`self.SetActorTickEnabled` true)
  (`KismetSystemLibrary.Delay` 1.0)
  (`self.SetActorTickEnabled` false)
  (set `MovementComponent.Velocity` (* (`KismetMathLibrary.Normal` (- PlayerPosition (`self.K2_GetActorLocation`))) 200.0) (`self.ProjectileMovement`)))

(event `self.ReceiveBeginPlay`
  (bind _outactors (`GameplayStatics.GetAllActorsOfClass` "/Game/BulletHell/BP_Pool.BP_Pool_C"))
  (set `self.Pool` (`KismetArrayLibrary.Array_Get` _outactors)))

(event `self.ReceiveTick`
  (params (DeltaSeconds :type "Float (single-precision)"))
  (bind _projectilemovement (`self.ProjectileMovement`))
  (bind _velocity (`MovementComponent.Velocity` _projectilemovement))
  (set `MovementComponent.Velocity` (+ _velocity (* (`KismetMathLibrary.Normal` _velocity) -10.0)) _projectilemovement))

(event `self.ReceiveHit`
  (params (MyComp :type "PrimitiveComponent Object Reference") (Other :type "Actor Object Reference") (OtherComp :type "PrimitiveComponent Object Reference") (bSelfMoved :type Boolean) (HitLocation :type "Vector Structure") (HitNormal :type "Vector Structure") (NormalImpulse :type "Vector Structure") (Hit :type "HitResult Structure (by ref)"))
  (bind _projectilemovement (`self.ProjectileMovement`))
  (`self.SetActorHiddenInGame` true)
  (`self.SetActorEnableCollision` false)
  (`ActorComponent.Deactivate` _projectilemovement)
  (`self.K2_SetActorLocation` (0.0 0.0 -1000.0) false true)
  (`self.SetActorTickEnabled` false)
  (set `MovementComponent.Velocity` (0.0 0.0 0.0) _projectilemovement)
  (`/Game/BulletHell/BP_Pool.AddBulletToPool` (`self.Pool`) self))

(event `self.ProjectileMovement.OnProjectileStop`
  (params (ImpactResult :type "HitResult Structure (by ref)"))
  (`MovementComponent.SetUpdatedComponent` (`self.ProjectileMovement`) (`self.Sphere`)))

(fn `ActivateBullet`
  (params (StartVelocity :type "Vector Structure") (SpawnLocation :type "Vector Structure"))
  (bind _projectilemovement (`self.ProjectileMovement`))
  (`self.SetActorHiddenInGame` false)
  (`self.SetActorEnableCollision` true)
  (`ActorComponent.Activate` _projectilemovement false)
  (`self.K2_SetActorLocation` SpawnLocation)
  (set `MovementComponent.Velocity` StartVelocity _projectilemovement))

(fn `UserConstructionScript`)