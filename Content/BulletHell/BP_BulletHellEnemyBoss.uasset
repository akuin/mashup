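; Bullet-hell boss that fights through five phases, each with its own bullet pattern and a full health bar.
; An authority-only looping timer feeds a gate that runs the current phase's pattern, drawing projectiles from a pool and often aiming or redirecting them at random players.
; Projectile hits route through RPCHit to MultiHit, which updates a circular health-bar material and handles phase changes with a brief invulnerable ceasefire, or the final explosion.
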(event `MultiPattern1`
  (bind _returnvalue (`self.K2_GetActorLocation`))
  (bind _shotbullets (`self.ShotBullets`))
  (bind _chance (`self.Chance`))
  (bind _turnvalue (`self.TurnValue`))
  (bind _returnvalue_2 (`KismetMathLibrary.RotateAngleAxis` (* (`KismetMathLibrary.Normal` (`KismetMathLibrary.MakeVector` 0.4 1.0)) 500.0) (* _turnvalue 70.0) (0.0 0.0 1.0)))
  (if (== _turnvalue 1.0)
    (set `self.TurnValue` 0.0))
  (if (== (`self.Chance`) 2.0)
    (set `self.Chance` 0.0))
  (bind _counter (`/Engine/EditorBlueprintResources/StandardMacros.Do N` 5 :!label _label)
    (:`Exit`
      (bind _bullet (`self.GetBulletAndActivate` _returnvalue _returnvalue_2)
        (:`Continue`
          (bind _bullet_2 (`self.GetBulletAndActivate` _returnvalue (`KismetMathLibrary.MirrorVectorByNormal` _returnvalue_2 (0.0 1.0 0.0)))
            (:`Continue`
              (`KismetArrayLibrary.Array_Add` _shotbullets _bullet)
              (`KismetArrayLibrary.Array_Add` _shotbullets _bullet_2)
              (if (== _counter 5)
                (set `self.TurnValue` (`KismetMathLibrary.FClamp` (+ (`self.TurnValue`) 0.2)))
                (set `self.Chance` (`KismetMathLibrary.FClamp` (+ _chance 0.3) 0.0 2.0))
                (for _array_element _shotbullets
                  (`/Game/BulletHell/BP_Projectile.SlowDown` _array_element (`KismetMathLibrary.VLerp` (`KismetMathLibrary.MakeVector` -5000.0) (`self.GetRandomPlayerPosition`) (`KismetMathLibrary.FClamp` _chance))))
                (`KismetArrayLibrary.Array_Clear` (`self.ShotBullets`))
                (goto _label :!via `Reset`)))))))))

(event `CloseGate`
  (bind _returnvalue (`self.K2_GetActorLocation`))
  (bind _returnvalue_2 (`self.K2_GetActorLocation`))
  (bind _returnvalue_3 (`KismetMathLibrary.MakeVector` 1.0))
  (bind _returnvalue_4 (`self.K2_GetActorLocation`))
  (bind _segments (`self.Segments`))
  (bind _shotbullets (`self.ShotBullets`))
  (bind _patternstruct_spawnpositions (break `/Game/BulletHell/PatternStruct` (make `/Game/BulletHell/PatternStruct` (`|MakeArray` (50.0 -5.0 0.0) (50.0 -2.5 0.0) (50.0 0.0 0.0) (50.0 2.5 0.0) (50.0 5.0 0.0) (80.0 -4.0 0.0) (80.0 -1.6 0.0) (80.0 1.6 0.0) (80.0 4.0 0.0) (110.0 -3.0 0.0) (110.0 0.0 0.0) (110.0 3.0 0.0) (140.0 -2.0 0.0) (140.0 2.0 0.0) :!type "Vector Structure"))))
  (bind _returnvalue_5 (`KismetMathLibrary.Normal` (- (+ (`self.GetRandomPlayerPosition`) (`KismetMathLibrary.MakeVector` (`KismetMathLibrary.RandomFloatInRange` -100.0 100.0) (`KismetMathLibrary.RandomFloatInRange` -100.0 100.0))) _returnvalue)))
  (goto _label_2 :!via `Toggle`))

(event `DoSomething`
  (bind _returnvalue (`self.K2_GetActorLocation`))
  (bind _returnvalue_2 (`self.K2_GetActorLocation`))
  (bind _returnvalue_3 (`KismetMathLibrary.MakeVector` 1.0))
  (bind _returnvalue_4 (`self.K2_GetActorLocation`))
  (bind _segments (`self.Segments`))
  (bind _shotbullets (`self.ShotBullets`))
  (bind _patternstruct_spawnpositions (break `/Game/BulletHell/PatternStruct` (make `/Game/BulletHell/PatternStruct` (`|MakeArray` (50.0 -5.0 0.0) (50.0 -2.5 0.0) (50.0 0.0 0.0) (50.0 2.5 0.0) (50.0 5.0 0.0) (80.0 -4.0 0.0) (80.0 -1.6 0.0) (80.0 1.6 0.0) (80.0 4.0 0.0) (110.0 -3.0 0.0) (110.0 0.0 0.0) (110.0 3.0 0.0) (140.0 -2.0 0.0) (140.0 2.0 0.0) :!type "Vector Structure"))))
  (bind _returnvalue_5 (`KismetMathLibrary.Normal` (- (+ (`self.GetRandomPlayerPosition`) (`KismetMathLibrary.MakeVector` (`KismetMathLibrary.RandomFloatInRange` -100.0 100.0) (`KismetMathLibrary.RandomFloatInRange` -100.0 100.0))) _returnvalue)))
  (`/Engine/EditorBlueprintResources/StandardMacros.Gate` false :!label _label_2
    (:`Exit`
      (switch `int` (`self.Phase`)
        (:`0`
          (`|ExecutionSequence`
            (:`then_0`
              (bind _counter (`/Engine/EditorBlueprintResources/StandardMacros.Do N` 40 :!label _label_3)
                (:`Exit`
                  (if (== _counter 40)
                    (`KismetSystemLibrary.Delay` 2.0)
                    (set `self.RandomFloat` (`KismetMathLibrary.RandomFloatInRange` -1.0 1.0))
                    (goto _label_3 :!via `Reset`)
                    (else
                      (bind _returnvalue_6 (/ (`KismetMathLibrary.Conv_IntToDouble` _counter) 40.0))
                      (bind _returnvalue_7 (* (`KismetMathLibrary.RotateAngleAxis` (`KismetMathLibrary.MakeVector` -1.0 (`self.RandomFloat`)) (* _returnvalue_6 360.0) (0.0 0.0 1.0)) 50.0))
                      (`self.GetBulletAndActivate` (+ (`self.K2_GetActorLocation`) _returnvalue_7) (* (`KismetMathLibrary.Normal` _returnvalue_7) (+ (* _returnvalue_6 300.0) 400.0))))))))
            (:`then_1`
              (`KismetSystemLibrary.Delay` 0.2)
              (bind (_projectile _issuccessful) (`/Game/BulletHell/BP_Pool.GetBulletFromPool` (`self.Pool`) true))
              (if _issuccessful
                (`/Game/BulletHell/BP_Projectile.ActivateBullet` _projectile (* _returnvalue_5 200.0) (+ (* _returnvalue_5 100.0) _returnvalue))))))
        (:`1`
          (`|ExecutionSequence`
            (:`then_0`
              (`KismetSystemLibrary.Delay` 0.5)
              (set `self.RandomLocation` (`KismetMathLibrary.MakeVector` (.x (`KismetMathLibrary.RandomUnitVector`)) (.y (`KismetMathLibrary.RandomUnitVector`))))
              (for _array_element _patternstruct_spawnpositions
                (bind _returnvalue_8 (`KismetMathLibrary.GreaterGreater_VectorRotator` _array_element (`KismetMathLibrary.FindLookAtRotation` _returnvalue_2 (+ _returnvalue_2 (`self.RandomLocation`)))))
                (`self.GetBulletAndActivate` (+ _returnvalue_8 _returnvalue_2) (* (`KismetMathLibrary.Normal` _returnvalue_8) 400.0))))
            (:`then_1`
              (`KismetSystemLibrary.Delay` 2.0)
              (`KismetArrayLibrary.Array_Clear` (`self.ShotBullets`))
              (for _index (range 1 (+ _segments 1))
                (bind _returnvalue_9 (`KismetMathLibrary.RotateAngleAxis` (* (`KismetMathLibrary.MakeVector` 1.0) 50.0) (* (/ (`KismetMathLibrary.Conv_IntToDouble` _index) (`KismetMathLibrary.Conv_IntToDouble` _segments)) 360.0) (0.0 0.0 1.0)))
                (bind _bullet (`self.GetBulletAndActivate` (+ _returnvalue_9 (`self.K2_GetActorLocation`)) (* (`KismetMathLibrary.Normal` _returnvalue_9) 200.0))
                  (:`Continue`
                    (`KismetArrayLibrary.Array_Add` (`self.ShotBullets`) _bullet))))
              (`KismetSystemLibrary.Delay` 1.0)
              (for _array_element_2 (`self.ShotBullets`)
                (`ProjectileMovementComponent.SetVelocityInLocalSpace` (`/Game/BulletHell/BP_Projectile.ProjectileMovement` _array_element_2) (* (`KismetMathLibrary.Normal` (- (`self.GetRandomPlayerPosition`) (`self.K2_GetActorLocation` _array_element_2))) 400.0))))))
        (:`2`
          (`KismetSystemLibrary.Delay` 0.25)
          (`self.MultiPattern1`))
        (:`3`
          (`KismetSystemLibrary.Delay` 0.6)
          (for _index_2 (range 1 9)
            (bind _returnvalue_10 (* (/ (`KismetMathLibrary.Conv_IntToDouble` _index_2) 8.0) 360.0))
            (`self.GetBulletAndActivate` _returnvalue_4 (`KismetMathLibrary.RotateAngleAxis` (* _returnvalue_3 500.0) (+ _returnvalue_10 (`KismetMathLibrary.RandomFloatInRange` -20.0 20.0)) (0.0 0.0 1.0))
              (:`Continue`
                (`self.GetBulletAndActivate` _returnvalue_4 (`KismetMathLibrary.SelectVector` (`KismetMathLibrary.RotateAngleAxis` (* _returnvalue_3 250.0) (+ _returnvalue_10 (`KismetMathLibrary.RandomFloatInRange` 10.0 30.0)) (0.0 0.0 1.0)) (* (`KismetMathLibrary.Normal` (- (`self.GetRandomPlayerPosition`) _returnvalue_4)) 250.0) (`KismetMathLibrary.RandomBoolWithWeight` 0.5)))))))
        (:`4`
          (`|ExecutionSequence`
            (:`then_0`
              (`/Engine/EditorBlueprintResources/StandardMacros.DoOnce` false
                (:`Completed`
                  _)))
            (:`then_1`
              (`KismetSystemLibrary.Delay` 6.0)))
          (for _ (range 1 151)
            (bind _bullet_2 (`self.GetBulletAndActivate` (`self.K2_GetActorLocation`) (* (`KismetMathLibrary.Normal` (`KismetMathLibrary.MakeVector` (.x (`KismetMathLibrary.RandomUnitVector`)) (.y (`KismetMathLibrary.RandomUnitVector`)))) (`KismetMathLibrary.RandomFloatInRange` 100.0 600.0)))
              (:`Continue`
                (`KismetArrayLibrary.Array_Add` (`self.ShotBullets`) _bullet_2))))
          (`KismetSystemLibrary.Delay` 1.5)
          (for _array_element_3 _shotbullets
            (if (`KismetArrayLibrary.Array_Contains` (`/Game/BulletHell/BP_Pool.ActiveBullets` (`self.Pool`)) _array_element_3)
              (`/Game/BulletHell/BP_Projectile.Freeze` _array_element_3)))
          (`KismetArrayLibrary.Array_Clear` _shotbullets))))))

(event `ActivateBoss`
  (`/Engine/EditorBlueprintResources/ActorMacros.Switch Has Authority` :!label _label_4
    (:`Authority`
      (bind _returnvalue (`KismetSystemLibrary.K2_SetTimerDelegate` (delegate `DoSomething`) 0.025 true)))))

(event `self.ReceiveBeginPlay`
  (`parent.ReceiveBeginPlay`)
  (bind _asui_circular_bar (cast `/Game/ProgressCircle/UI_CircularBar` (`WidgetComponent.GetUserWidgetObject` (`self.Widget`))))
  (bind _returnvalue (`Image.GetDynamicMaterial` (`/Game/ProgressCircle/UI_CircularBar.Image_117` _asui_circular_bar)))
  (set `self.HealthBarMaterial` _returnvalue)
  (`MaterialInstanceDynamic.SetScalarParameterValue` _returnvalue "Alpha" 1.0)
  (goto _label_4))

(event `self.ReceiveTick`
  (params (DeltaSeconds :type "Float (single-precision)")))

(event `RPCHit`
  (`self.MultiHit`))

(event `MultiHit`
  (bind _phase (`self.Phase`))
  (if (not (`self.Invulnerable`))
    (bind _result (`/Engine/EditorBlueprintResources/StandardMacros.DecrementFloat` (`self.Health`))
      (:`  `
        (bind _output_get (set `self.Health` _result))
        (`MaterialInstanceDynamic.SetScalarParameterValue` (`self.HealthBarMaterial`) "Alpha" (/ _output_get 100.0))
        (if (<= _output_get 0.0)
          (if (== _phase 4)
            (`GameplayStatics.SpawnEmitterAtLocation` "/Game/Effects/Particle_Systems/P_Explosion_Fireball.P_Explosion_Fireball")
            (`KismetSystemLibrary.K2_ClearAndInvalidateTimerHandle` (stale `ActivateBoss` _returnvalue))
            (`self.SetActorHiddenInGame` true)
            (`self.SetActorEnableCollision` false)
            (set `self.Phase` 100)
            (else
              (`/Engine/EditorBlueprintResources/StandardMacros.IncrementInt` _phase
                (:`  `
                  (set `self.Health` 100.0)
                  (`self.CloseGate`)
                  (set `self.Invulnerable` true)
                  (`KismetSystemLibrary.Delay` 4.0)
                  (`self.CloseGate`)
                  (set `self.Invulnerable` false)
                  (`MaterialInstanceDynamic.SetScalarParameterValue` (`self.HealthBarMaterial`) "Alpha" 1.0))))))))))

(event `self.ReceiveHit`
  (params (MyComp :type "PrimitiveComponent Object Reference") (Other :type "Actor Object Reference") (OtherComp :type "PrimitiveComponent Object Reference") (bSelfMoved :type Boolean) (HitLocation :type "Vector Structure") (HitNormal :type "Vector Structure") (NormalImpulse :type "Vector Structure") (Hit :type "HitResult Structure (by ref)"))
  (if (`KismetMathLibrary.ClassIsChildOf` (`GameplayStatics.GetObjectClass` Other) "/Game/BulletHell/BP_Projectile.BP_Projectile_C")
    (`self.RPCHit`)))

(event `self.Shoot`
  (bind _returnvalue (`self.K2_GetActorLocation`))
  (bind _playerlist (`self.PlayerList`))
  (bind _radius (`self.Radius`))
  (switch `int` 0
    (:`Default`
      (bind (_projectile _issuccessful) (`/Game/BulletHell/BP_Pool.GetBulletFromPool` (`self.Pool`) true :!label _label_5))
      (if _issuccessful
        (bind _returnvalue_2 (`KismetMathLibrary.Conv_IntToDouble` (stale _index)))
        (`/Game/BulletHell/BP_Projectile.ActivateBullet` _projectile (* (`KismetMathLibrary.Normal` (- (`self.K2_GetActorLocation` (`|GetArrayItem` _playerlist (`KismetMathLibrary.RandomIntegerInRange` 0 (- (`KismetArrayLibrary.Array_Length` _playerlist) 1)))) _returnvalue)) 500.0) (+ (`KismetMathLibrary.MakeVector` (* _radius (`KismetMathLibrary.Sin` _returnvalue_2)) (* _radius (`KismetMathLibrary.Cos` _returnvalue_2))) _returnvalue))))
    (:`0`
      (for _index (range 1 (+ (`self.Segments`) 1))
        (goto _label_5)))))

(fn `UserConstructionScript`
  (`parent.UserConstructionScript`)
  (set `self.Health` 100.0))